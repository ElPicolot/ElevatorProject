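; BP_ControlPanel is an elevator control panel that builds one numbered button per floor at BeginPlay.
; It adds mesh components in a wrapping grid from a start position, each tagged as an elevator button with a zero-based floor index.
; Each button gets a text label showing the one-based floor number.
; The same loop tells the referenced elevator's call button to spawn a button for that floor.
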(event EventBeginPlay
  (Variables|Default|SetControl%20Panel%20Button%20OffsetCache (Variables|ControlPanelButtons|GetControlPanelButtonOffset))
  (Variables|Default|SetMax%20Horizontal%20ButtonsCache (Variables|ControlPanelButtons|GetMaxHorizontalButtons))
  (Variables|Default|SetStartTransform (Transformation|GetRelativeTransform (Variables|Default|GetStartPosition)))
  (for _index (range 1 (Variables|Default|GetNumberOfFloors))
    (Variables|Default|SetCurrentLineValue _index)
    (if (> (Variables|Default|GetCurrentLineValue) (Variables|ControlPanelButtons|GetMaxHorizontalButtons))
      (Variables|Default|SetNewLineValue (+ (Variables|Default|GetNewLineValue) (Variables|Default|GetControlPanelButtonDistanceBetwenvVer)))
      (Variables|ControlPanelButtons|SetControlPanelButtonOffset (Variables|Default|GetControl%20Panel%20Button%20OffsetCache))
      (Variables|ControlPanelButtons|SetMaxHorizontalButtons (+ (Variables|ControlPanelButtons|GetMaxHorizontalButtons) (Variables|Default|GetMax%20Horizontal%20ButtonsCache))))
    (bind _returnvalue (AddComponent|AddStaticMeshComponent false (Variables|Default|GetStartTransform)))
    (bind _output_get (Variables|Default|SetButtonMeshCompRef _returnvalue))
    (Variables|/Script/Engine.ActorComponent|SetComponentTags _output_get (Utilities|Array|MakeArray "ElevatorButton" (Utilities|String|StringToName (Utilities|String|ToString(Integer) (- (Variables|Default|GetCurrentLineValue) 1)))))
    (Transformation|SetRelativeLocation (Variables|Default|GetButtonMeshCompRef) (Math|Vector|MakeVector (.x (.location (Variables|Default|GetStartTransform))) (- (Variables|ControlPanelButtons|GetControlPanelButtonOffset) (.y (.location (Variables|Default|GetStartTransform)))) (- (.z (.location (Variables|Default|GetStartTransform))) (Variables|Default|GetNewLineValue))) false false)
    (Variables|ControlPanelButtons|SetControlPanelButtonOffset (- (Variables|ControlPanelButtons|GetControlPanelButtonOffset) (Variables|Default|GetControlPanelButtonDistanceBetwenHor)))
    (Default|SpawnButton (Variables|/Game/ElevatorSystem/BP_Elevator.BP_Elevator_C|GetElevatorCallButtonRef (Variables|Default|GetElevatorRef)) (Utilities|String|StringToName (Utilities|String|ToString(Integer) (- (Variables|Default|GetCurrentLineValue) 1))))
    (bind _returnvalue_2 (AddComponent|AddTextRenderComponent false (Math|Transform|MakeTransform (Math|Vector|MakeVector (.x (Variables|/Script/Engine.SceneComponent|GetRelativeLocation (Variables|Default|GetButtonMeshCompRef))) (.y (Variables|/Script/Engine.SceneComponent|GetRelativeLocation (Variables|Default|GetButtonMeshCompRef))) (.z (Variables|/Script/Engine.SceneComponent|GetRelativeLocation (Variables|Default|GetButtonMeshCompRef)))) "0, 0, 0" "1.000000,1.000000,1.000000")))
    (Rendering|Components|TextRender|SetText _returnvalue_2 (Utilities|Text|ToText(Integer) (+ (Math|Conversions|ToInteger(Byte) (Utilities|String|ToString(Text) (Utilities|Text|ToText(Name) (Utilities|String|StringToName (Utilities|String|ToString(Integer) (- (Variables|Default|GetCurrentLineValue) 1)))))) 1)))))

(fn ConstructionScript)