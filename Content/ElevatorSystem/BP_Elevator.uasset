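; Elevator actor that spawns a call button and an attached floor control panel at BeginPlay, handing both a reference to itself.
; GoToFloorEvent ignores requests while active, otherwise opens or closes the doors depending on whether the target is the current floor.
; ElevatorUp and ElevatorDown share a timeline that lerps height to floor times floor height, then reopens the doors.
; A second timeline animates both doors by scaling their Y axis.
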(event Custom|GoToFloorEvent
  (params (Floor :type Integer))
  (if (not (Variables|Default|GetCurrentlyActive?))
    (Variables|Default|SetFloorToRef Floor)
    (if (== (Variables|Default|GetFloorToRef) (Variables|Default|GetWhatFloorWeAt?))
      (Development|PrintString (Utilities|String|Append "Already At Floor:" (Utilities|String|ToString(Integer) (Variables|Default|GetFloorToRef)) "" "Opening doors"))
      (CallFunction|OpenCloseElevatorDoor true)
      (Utilities|FlowControl|Delay (Components|Animation|GetPlayRate (Variables|Default|GetOpenCloseElevatorDoorTimeline)))
      (if (> (Variables|Default|GetFloorToRef) (Variables|Default|GetWhatFloorWeAt?))
        (CallFunction|ElevatorUp)
        (else
          (CallFunction|ElevatorDown)))
      (else
        (Variables|Default|SetCurrentlyActive? true)
        (Development|PrintString (Utilities|String|Append "Going To Floor:" (Utilities|String|ToString(Integer) (Variables|Default|GetFloorToRef)) "" "Closing the doors"))
        (CallFunction|OpenCloseElevatorDoor false)))))

(event Custom|OpenCloseElevatorDoor
  (params (Open? :type Boolean))
  (bind _door2 (Variables|Default|GetDoor2))
  (bind _relativescale3d (Variables|/Script/Engine.SceneComponent|GetRelativeScale3D _door2))
  (Components|Timeline|SetPlayRate (Variables|Default|GetOpenCloseElevatorDoorTimeline) (/ 1.0 (Variables|Default|GetElevatorDoorSpeed)))
  (if Open?
    (bind _opencloseelevatordoorfloattrack (Timeline|OpenCloseElevatorDoorTimeline PlayFromStart)
      (:Update
        (Transformation|SetRelativeScale3D (Variables|Default|GetDoor1) (Math|Vector|MakeVector (.x _relativescale3d) (Math|Float|Lerp 1.1 0.1 _opencloseelevatordoorfloattrack) (.z _relativescale3d)))))
    (else
      (Timeline|OpenCloseElevatorDoorTimeline ReverseFromEnd))))

(event Custom|ElevatorUp
  (bind _returnvalue (Transformation|GetActorLocation))
  (Components|Timeline|SetPlayRate (Variables|Default|GetGoingUpDownTimeline) (/ (/ 1.0 (Variables|Default|GetElevatorSpeed)) (Variables|Default|GetFloorToRef)))
  (Variables|Default|SetStartZ (.z (Transformation|GetActorLocation)))
  (bind _goingupdowntimelinefloattrack (Timeline|GoingUpDownTimeline PlayFromStart)
    (:Update
      (Transformation|SetActorLocation (Math|Vector|MakeVector (.x _returnvalue) (.y _returnvalue) (Math|Float|Lerp (Variables|Default|GetStartZ) (Math|Conversions|ToFloat(Integer) (* (Variables|Default|GetFloorToRef) (Math|Float|Truncate (Variables|Floors|GetFloorHeight)))) _goingupdowntimelinefloattrack)) false false))
    (:Finished
      (Variables|Default|SetStartZ (.z (Transformation|GetActorLocation)))
      (Variables|Default|SetWhatFloorWeAt? (Variables|Default|GetFloorToRef))
      (CallFunction|OpenCloseElevatorDoor true)
      (Utilities|FlowControl|Delay (Components|Animation|GetPlayRate (Variables|Default|GetOpenCloseElevatorDoorTimeline)))
      (Variables|Default|SetCurrentlyActive? false))))

(event Custom|ElevatorDown
  (bind _returnvalue (Transformation|GetActorLocation))
  (Components|Timeline|SetPlayRate (Variables|Default|GetGoingUpDownTimeline) (/ (/ 1.0 (Variables|Default|GetElevatorSpeed)) (Math|Conversions|ToFloat(Integer) (- (Variables|Default|GetWhatFloorWeAt?) (Variables|Default|GetFloorToRef)))))
  (Variables|Default|SetStartZ (.z (Transformation|GetActorLocation)))
  (bind _goingupdowntimelinefloattrack (Timeline|GoingUpDownTimeline PlayFromStart)
    (:Update
      (Transformation|SetActorLocation (Math|Vector|MakeVector (.x _returnvalue) (.y _returnvalue) (Math|Float|Lerp (Variables|Default|GetStartZ) (Math|Conversions|ToFloat(Integer) (* (Variables|Default|GetFloorToRef) (Math|Float|Truncate (Variables|Floors|GetFloorHeight)))) _goingupdowntimelinefloattrack)) false false))
    (:Finished
      (Variables|Default|SetStartZ (.z (Transformation|GetActorLocation)))
      (Variables|Default|SetWhatFloorWeAt? (Variables|Default|GetFloorToRef))
      (CallFunction|OpenCloseElevatorDoor true)
      (Utilities|FlowControl|Delay (Components|Animation|GetPlayRate (Variables|Default|GetOpenCloseElevatorDoorTimeline)))
      (Variables|Default|SetCurrentlyActive? false))))

(event EventBeginPlay
  (bind _controlpanelarrow (Variables|Default|GetControlPanelArrow))
  (bind _returnvalue (Transformation|GetWorldLocation _controlpanelarrow))
  (bind _returnvalue_2 (Game|SpawnActorfromClass "/Game/ElevatorSystem/BP_ElevatorCallButton.BP_ElevatorCallButton_C" (Math|Transform|MakeTransform (.location (Transformation|GetWorldTransform (Variables|Default|GetButtonArrow))) "0, 0, 0" "1.000000,1.000000,1.000000") "Undefined" "MultiplyWithRoot" 0 (Variables|CallButton|GetCall%20Button%20Vert%20Offset) (Variables|CallButton|GetCall%20Button%20Hor%20Offset) (Variables|CallButton|GetCall%20Button%20Depth%20Offset) (Variables|CallButton|GetCall%20Button%20Mesh) self 0))
  (Variables|Default|SetElevatorCallButtonRef _returnvalue_2)
  (bind _returnvalue_3 (Game|SpawnActorfromClass "/Game/ElevatorSystem/BP_ControlPanel.BP_ControlPanel_C" (Math|Transform|MakeTransform (Math|Vector|MakeVector (+ (.x _returnvalue) (Variables|CallButton|GetCall%20Button%20Depth%20Offset)) (+ (.y _returnvalue) (Variables|ControlPanelPanel|GetControlPanelHorOffset)) (+ (.z _returnvalue) (Variables|ControlPanelPanel|GetControlPanelVertOffset))) "0, 0, 0" "1.000000,1.000000,1.000000") "Undefined" "MultiplyWithRoot" 0 (Variables|ElevatorControlPanel|GetControl%20Panel%20Button%20Offset) (Variables|ElevatorControlPanel|GetMax%20Horizontal%20Buttons) (Variables|Floors|GetNumber%20Of%20Floors) (Variables|ElevatorControlPanel|GetControl%20Panel%20Button%20Distance%20Betwen%20Hor) (Variables|ElevatorControlPanel|GetControl%20Panel%20Button%20Distance%20Betwenv%20Ver) self 0))
  (Transformation|AttachActorToActor _returnvalue_3 self "None" "KeepWorld" "KeepWorld" "KeepWorld" true))

(fn ConstructionScript)